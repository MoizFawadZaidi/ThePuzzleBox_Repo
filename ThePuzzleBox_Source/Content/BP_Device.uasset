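; BP_Device is a trigger device that opens a sliding door while a holdable item overlaps its box.
; Begin overlap with BP_Holdable_ItemA, B or C finds the first BP_SlidingDoor via GetActorOfClass and calls OpenDoors.
; End overlap with any of those items calls CloseDoors the same way, without tracking whether other items remain inside.
; Both events print an activation debug message.
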(event OnComponentBeginOverlap(Box)
  (params (OverlappedComponent :type Primitive%20Component%20Object%20Reference) (OtherActor :type Actor%20Object%20Reference) (OtherComp :type Primitive%20Component%20Object%20Reference) (OtherBodyIndex :type Integer) (bFromSweep :type Boolean) (SweepResult :type Hit%20Result%20Structure%20%28by%20ref%29))
  (Utilities|FlowControl|Sequence
    (:then_0
      (Utilities|Casting|CastToBP_Holdable_ItemA OtherActor))
    (:then_1
      (Utilities|Casting|CastToBP_Holdable_ItemB OtherActor))
    (:then_2
      (Utilities|Casting|CastToBP_Holdable_ItemC OtherActor)))
  (Development|PrintString "Activated")
  (bind _returnvalue (Actor|GetActorOfClass "/Game/BP_SlidingDoor.BP_SlidingDoor_C"))
  (Default|OpenDoors _returnvalue))

(event OnComponentEndOverlap(Box)
  (params (OverlappedComponent :type Primitive%20Component%20Object%20Reference) (OtherActor :type Actor%20Object%20Reference) (OtherComp :type Primitive%20Component%20Object%20Reference) (OtherBodyIndex :type Integer))
  (Utilities|FlowControl|Sequence
    (:then_0
      (Utilities|Casting|CastToBP_Holdable_ItemA OtherActor))
    (:then_1
      (Utilities|Casting|CastToBP_Holdable_ItemB OtherActor))
    (:then_2
      (Utilities|Casting|CastToBP_Holdable_ItemC OtherActor)))
  (Development|PrintString "De-activated")
  (bind _returnvalue (Actor|GetActorOfClass "/Game/BP_SlidingDoor.BP_SlidingDoor_C"))
  (Default|CloseDoors _returnvalue))

(fn ConstructionScript)