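; Pressure plate that opens a sliding door while the player character or a held-type flashlight item rests on it.
; Box overlap events track the character and flashlight weights as separate booleans, so the door closes only when both are gone.
; The plate material switches between blue glow and grey, and the door is found by class lookup of BP_SlidingDoorB1.
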(event OnComponentBeginOverlap(Box)
  (params (OverlappedComponent :type Primitive%20Component%20Object%20Reference) (OtherActor :type Actor%20Object%20Reference) (OtherComp :type Primitive%20Component%20Object%20Reference) (OtherBodyIndex :type Integer) (bFromSweep :type Boolean) (SweepResult :type Hit%20Result%20Structure%20%28by%20ref%29))
  (Utilities|FlowControl|Sequence
    (:then_0
      (Utilities|Casting|CastToBP_CharacterB OtherActor)
      (Variables|Default|SetIsCharaWeight? true))
    (:then_1
      (Utilities|Casting|CastToBP_Holdable_ItemB_Flashlight OtherActor)
      (Variables|Default|SetIsFlashlightWeight? true)))
  (Rendering|Material|SetMaterial (Variables|Default|GetPlate) 0 "/Game/Materials/M_BlueGlow.M_BlueGlow")
  (bind _returnvalue (Actor|GetActorOfClass "/Game/SlidingDoors/BP_SlidingDoorB1.BP_SlidingDoorB1_C"))
  (Default|OpenDoors _returnvalue))

(event OnComponentEndOverlap(Box)
  (params (OverlappedComponent :type Primitive%20Component%20Object%20Reference) (OtherActor :type Actor%20Object%20Reference) (OtherComp :type Primitive%20Component%20Object%20Reference) (OtherBodyIndex :type Integer))
  (Utilities|FlowControl|Sequence
    (:then_0
      (Utilities|Casting|CastToBP_CharacterB OtherActor)
      (Variables|Default|SetIsCharaWeight? false)
      (if (not (Variables|Default|GetIsFlashlightWeight?))
        (Rendering|Material|SetMaterial (Variables|Default|GetPlate) 0 "/Game/Materials/M_Grey.M_Grey" :!label _label)
        (bind _returnvalue (Actor|GetActorOfClass "/Game/SlidingDoors/BP_SlidingDoorB1.BP_SlidingDoorB1_C"))
        (Default|CloseDoors _returnvalue)))
    (:then_1
      (Utilities|Casting|CastToBP_Holdable_ItemB_Flashlight OtherActor)
      (Variables|Default|SetIsFlashlightWeight? false)
      (if (not (Variables|Default|GetIsCharaWeight?))
        (goto _label)))))

(fn ConstructionScript)