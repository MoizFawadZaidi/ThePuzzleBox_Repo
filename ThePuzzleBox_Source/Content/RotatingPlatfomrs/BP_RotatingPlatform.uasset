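; BP_RotatingPlatform is a platform actor that rotates while a device is active.
; Each tick it looks up BP_CharacterB and BP_DeviceB, playing the Rotating timeline when the device is activated and the character has no battery attached, otherwise stopping it.
; The timeline's RotationTrack value is added as a local pitch delta on every update, so the track sets the per-frame step rather than an absolute angle.
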(event Custom|Stop%20Timeline
  (bind _rotation_track (Timeline|Rotating Stop)
    (:Update
      (Transformation|AddActorLocalRotation (Math|Rotator|MakeRotator 0.0 _rotation_track 0.0) false false))))

(event Custom|Play%20Timeline
  (bind _rotation_track (Timeline|Rotating Play)
    (:Update
      (Transformation|AddActorLocalRotation (Math|Rotator|MakeRotator 0.0 _rotation_track 0.0) false false))))

(event EventTick
  (params (DeltaSeconds :type Float%20%28single-precision%29))
  (bind _returnvalue (Actor|GetActorOfClass "/Game/FirstPerson/Blueprints/BP_CharacterB.BP_CharacterB_C"))
  (if (Variables|/Game/FirstPerson/Blueprints/BP_CharacterB.BP_CharacterB_C|GetIsBatteryItemAttached? _returnvalue)
    (CallFunction|StopTimeline)
    (else
      (bind _returnvalue_2 (Actor|GetActorOfClass "/Game/Machines/BP_DeviceB.BP_DeviceB_C"))
      (if (Variables|/Game/Machines/BP_DeviceB.BP_DeviceB_C|GetDeviceActivated? _returnvalue_2)
        (CallFunction|PlayTimeline)
        (else
          (CallFunction|StopTimeline))))))

(fn ConstructionScript)