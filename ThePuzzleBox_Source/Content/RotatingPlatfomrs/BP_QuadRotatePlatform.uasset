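; BP_QuadRotatePlatform is a puzzle platform actor that spins on a self-restarting yaw timeline, started and stopped through custom events.
; Every Tick it checks whether the owl and coffee activators overlap their platform meshes while BP_ColorChangerDevice reports a correct combo.
; The owl check plays or reverses BP_GateB.
; The coffee check updates IsCoffeeGreen and opens BP_SlidingDoorC2 if BP_Contraption's left green is also active, with all actors found via GetActorOfClass.
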(event Custom|Stop%20Timeline
  (bind _rotation_track (Timeline|Timeline Stop)
    (:Update
      (Transformation|AddActorLocalRotation (Math|Rotator|MakeRotator 0.0 0.0 _rotation_track) false false))
    (:Finished
      (CallFunction|PlayTimeline))))

(event Custom|Play%20Timeline
  (bind _rotation_track (Timeline|Timeline Play)
    (:Update
      (Transformation|AddActorLocalRotation (Math|Rotator|MakeRotator 0.0 0.0 _rotation_track) false false))
    (:Finished
      (CallFunction|PlayTimeline))))

(event EventTick
  (params (DeltaSeconds :type Float%20%28single-precision%29))
  (Utilities|FlowControl|Sequence
    (:then_0
      (bind _returnvalue (Actor|GetActorOfClass "/Game/BP_OwlActivator.BP_OwlActivator_C"))
      (if (Collision|IsOverlappingActor (Variables|Default|GetSM_OwlPlatform) _returnvalue :!class /Script/Engine.PrimitiveComponent)
        (bind _returnvalue_2 (Actor|GetActorOfClass "/Game/BP_ColorChangerDevice.BP_ColorChangerDevice_C"))
        (if (Variables|/Game/BP_ColorChangerDevice.BP_ColorChangerDevice_C|GetCorrectCombo _returnvalue_2)
          (bind _returnvalue_3 (Actor|GetActorOfClass "/Game/BP_GateB.BP_GateB_C"))
          (Default|PlayTimeline _returnvalue_3)
          (else
            (bind _returnvalue_4 (Actor|GetActorOfClass "/Game/BP_GateB.BP_GateB_C"))
            (Default|ReverseTimeline _returnvalue_4)))
        (else
          (bind _returnvalue_5 (Actor|GetActorOfClass "/Game/BP_GateB.BP_GateB_C"))
          (Default|ReverseTimeline _returnvalue_5))))
    (:then_1
      (bind _returnvalue_6 (Actor|GetActorOfClass "/Game/BP_CoffeeActivator.BP_CoffeeActivator_C"))
      (if (Collision|IsOverlappingActor (Variables|Default|GetSM_CoffeePlatform) _returnvalue_6 :!class /Script/Engine.PrimitiveComponent)
        (bind _returnvalue_7 (Actor|GetActorOfClass "/Game/BP_ColorChangerDevice.BP_ColorChangerDevice_C"))
        (if (Variables|/Game/BP_ColorChangerDevice.BP_ColorChangerDevice_C|GetCorrectCombo _returnvalue_7)
          (Variables|Default|SetIsCoffeeGreen? true)
          (bind _returnvalue_8 (Actor|GetActorOfClass "/Game/Machines/BP_Contraption.BP_Contraption_C"))
          (if (Variables|/Game/Machines/BP_Contraption.BP_Contraption_C|GetLeftGreenActivated? _returnvalue_8)
            (bind _returnvalue_9 (Actor|GetActorOfClass "/Game/SlidingDoors/BP_SlidingDoorC2.BP_SlidingDoorC2_C"))
            (Default|OpenDoors _returnvalue_9)
            (else
              (bind _returnvalue_10 (Actor|GetActorOfClass "/Game/SlidingDoors/BP_SlidingDoorC2.BP_SlidingDoorC2_C"))
              (Default|CloseDoors _returnvalue_10)))
          (else
            (Variables|Default|SetIsCoffeeGreen? false)
            (bind _returnvalue_11 (Actor|GetActorOfClass "/Game/SlidingDoors/BP_SlidingDoorC2.BP_SlidingDoorC2_C"))
            (Default|CloseDoors _returnvalue_11)))
        (else
          (bind _returnvalue_12 (Actor|GetActorOfClass "/Game/SlidingDoors/BP_SlidingDoorC2.BP_SlidingDoorC2_C"))
          (Default|CloseDoors _returnvalue_12))))))

(fn ConstructionScript)