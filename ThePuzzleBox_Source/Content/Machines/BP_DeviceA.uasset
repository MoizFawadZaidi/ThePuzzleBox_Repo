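; BP_DeviceA is a battery-powered switch that toggles which of two sliding doors, pink or blue, is open.
; Interacting flip-flops the color state and cylinder glow material, switching doors only while the device is powered.
; A BatteryA item entering the box powers it and opens the selected door; removing it closes both.
; Doors are found by class with GetActorOfClass, so each color drives one BP_SlidingDoorA or BP_SlidingDoorB2 instance.
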(event OnComponentBeginOverlap(Box)
  (params (OverlappedComponent :type Primitive%20Component%20Object%20Reference) (OtherActor :type Actor%20Object%20Reference) (OtherComp :type Primitive%20Component%20Object%20Reference) (OtherBodyIndex :type Integer) (bFromSweep :type Boolean) (SweepResult :type Hit%20Result%20Structure%20%28by%20ref%29))
  (Utilities|Casting|CastToBP_Holdable_Item_BatteryA OtherActor)
  (Variables|Default|SetDeviceActivated? true)
  (if (Variables|Default|GetPinkActivated?)
    (CallFunction|OPENPinkCLOSEBlue)
    (else
      (CallFunction|OPENBlueCLOSEPink))))

(event OnComponentEndOverlap(Box)
  (params (OverlappedComponent :type Primitive%20Component%20Object%20Reference) (OtherActor :type Actor%20Object%20Reference) (OtherComp :type Primitive%20Component%20Object%20Reference) (OtherBodyIndex :type Integer))
  (Utilities|Casting|CastToBP_Holdable_Item_BatteryA OtherActor)
  (Variables|Default|SetDeviceActivated? false)
  (Utilities|FlowControl|Sequence
    (:then_0
      (bind _returnvalue (Actor|GetActorOfClass "/Game/SlidingDoors/BP_SlidingDoorB2.BP_SlidingDoorB2_C"))
      (Default|CloseDoors _returnvalue))
    (:then_1
      (bind _returnvalue_2 (Actor|GetActorOfClass "/Game/SlidingDoors/BP_SlidingDoorA.BP_SlidingDoorA_C"))
      (Default|CloseDoors _returnvalue_2))))

(event Custom|OPEN%20blue%20CLOSE%20pink
  (bind _returnvalue (Actor|GetActorOfClass "/Game/SlidingDoors/BP_SlidingDoorB2.BP_SlidingDoorB2_C"))
  (Default|OpenDoors _returnvalue)
  (Utilities|IsValid (stale Custom|OPEN%20pink%20CLOSE%20blue _returnvalue)
    (:Is%20Valid
      (Default|CloseDoors (stale Custom|OPEN%20pink%20CLOSE%20blue _returnvalue)))))

(event Custom|OPEN%20pink%20CLOSE%20blue
  (bind _returnvalue (Actor|GetActorOfClass "/Game/SlidingDoors/BP_SlidingDoorA.BP_SlidingDoorA_C"))
  (Default|OpenDoors _returnvalue)
  (Utilities|IsValid (stale Custom|OPEN%20blue%20CLOSE%20pink _returnvalue)
    (:Is%20Valid
      (Default|CloseDoors (stale Custom|OPEN%20blue%20CLOSE%20pink _returnvalue)))))

(event EventInteract
  (bind _deviceactivated_ (Variables|Default|GetDeviceActivated?))
  (bind _cylinder (Variables|Default|GetCylinder))
  (Utilities|FlowControl|FlipFlop
    (:A
      (Variables|Default|SetPinkActivated? false)
      (Variables|Default|SetBlueActivated? true)
      (Rendering|Material|SetMaterial _cylinder 0 "/Game/Materials/M_BlueGlow.M_BlueGlow")
      (if _deviceactivated_
        (CallFunction|OPENBlueCLOSEPink)))
    (:B
      (Variables|Default|SetBlueActivated? false)
      (Variables|Default|SetPinkActivated? true)
      (Rendering|Material|SetMaterial _cylinder 0 "/Game/Materials/M_PinkGlow.M_PinkGlow")
      (if _deviceactivated_
        (CallFunction|OPENPinkCLOSEBlue)))))

(fn ConstructionScript)