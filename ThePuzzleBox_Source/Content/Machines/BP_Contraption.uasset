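; Puzzle contraption with green, pink and blue pressure plates that react to BP_Holdable_Item overlaps by swapping glow materials and driving other level actors.
; Left green only sets its flag; right green triggers BP_DeviceB's open/close logic and closes BP_SlidingDoorC1 on release.
; Pink lights BP_DeviceA1 and plays BP_GateA's timeline if that device is active, reversing on release; blue toggles BP_Lights.
; Targets are found by GetActorOfClass, assuming one instance each.
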(event OnComponentBeginOverlap(GreenPlate_Collision)
  (params (OverlappedComponent :type Primitive%20Component%20Object%20Reference) (OtherActor :type Actor%20Object%20Reference) (OtherComp :type Primitive%20Component%20Object%20Reference) (OtherBodyIndex :type Integer) (bFromSweep :type Boolean) (SweepResult :type Hit%20Result%20Structure%20%28by%20ref%29))
  ;[0.07778 1 0] Green
  (Utilities|Casting|CastToBP_Holdable_ItemC OtherActor)
  (Rendering|Material|SetMaterial (Variables|Default|GetSM_GreenPlate) 0 "/Game/Materials/M_GreenGlow.M_GreenGlow")
  (Variables|Default|SetLeftGreenActivated? true))

(event OnComponentBeginOverlap(GreenPlate2_Collision)
  (params (OverlappedComponent :type Primitive%20Component%20Object%20Reference) (OtherActor :type Actor%20Object%20Reference) (OtherComp :type Primitive%20Component%20Object%20Reference) (OtherBodyIndex :type Integer) (bFromSweep :type Boolean) (SweepResult :type Hit%20Result%20Structure%20%28by%20ref%29))
  ;[0.07778 1 0] Green
  (Utilities|Casting|CastToBP_Holdable_ItemC OtherActor)
  (Rendering|Material|SetMaterial (Variables|Default|GetSM_GreenPlate2) 0 "/Game/Materials/M_GreenGlow.M_GreenGlow")
  (Variables|Default|SetRightGreenActivated? true)
  (bind _returnvalue (Actor|GetActorOfClass "/Game/Machines/BP_DeviceB.BP_DeviceB_C"))
  (if (Variables|/Game/Machines/BP_DeviceB.BP_DeviceB_C|GetGreenActivated? _returnvalue)
    (Default|OPENGreenCLOSEBlue _returnvalue)
    (elif (Variables|/Game/Machines/BP_DeviceB.BP_DeviceB_C|GetBlueActivated? _returnvalue)
      (Default|OPENBlueCLOSEGreen _returnvalue))))

(event OnComponentEndOverlap(GreenPlate_Collision)
  (params (OverlappedComponent :type Primitive%20Component%20Object%20Reference) (OtherActor :type Actor%20Object%20Reference) (OtherComp :type Primitive%20Component%20Object%20Reference) (OtherBodyIndex :type Integer))
  ;[0.07778 1 0] Green
  (Utilities|Casting|CastToBP_Holdable_ItemC OtherActor)
  (Rendering|Material|SetMaterial (Variables|Default|GetSM_GreenPlate) 0 "/Game/Materials/M_Grey.M_Grey")
  (Variables|Default|SetLeftGreenActivated? false))

(event OnComponentEndOverlap(GreenPlate2_Collision)
  (params (OverlappedComponent :type Primitive%20Component%20Object%20Reference) (OtherActor :type Actor%20Object%20Reference) (OtherComp :type Primitive%20Component%20Object%20Reference) (OtherBodyIndex :type Integer))
  ;[0.07778 1 0] Green
  (Utilities|Casting|CastToBP_Holdable_ItemC OtherActor)
  (Rendering|Material|SetMaterial (Variables|Default|GetSM_GreenPlate2) 0 "/Game/Materials/M_Grey.M_Grey")
  (Variables|Default|SetRightGreenActivated? false)
  (bind _returnvalue (Actor|GetActorOfClass "/Game/SlidingDoors/BP_SlidingDoorC1.BP_SlidingDoorC1_C"))
  (Default|CloseDoors _returnvalue))

(event OnComponentBeginOverlap(PinkPlate_Collision)
  (params (OverlappedComponent :type Primitive%20Component%20Object%20Reference) (OtherActor :type Actor%20Object%20Reference) (OtherComp :type Primitive%20Component%20Object%20Reference) (OtherBodyIndex :type Integer) (bFromSweep :type Boolean) (SweepResult :type Hit%20Result%20Structure%20%28by%20ref%29))
  ;[1 0.2604 0.5964] Pink
  (Utilities|Casting|CastToBP_Holdable_ItemC OtherActor)
  (Rendering|Material|SetMaterial (Variables|Default|GetSM_PinkPlate) 0 "/Game/Materials/M_PinkGlow.M_PinkGlow")
  (bind _returnvalue (Actor|GetActorOfClass "/Game/Machines/BP_DeviceA1.BP_DeviceA1_C"))
  (Rendering|Material|SetMaterial (Variables|/Game/Machines/BP_DeviceA1.BP_DeviceA1_C|GetCylinder _returnvalue) 0 "/Game/Materials/M_PinkGlow.M_PinkGlow")
  (Variables|Default|SetPinkActivated? true)
  (bind _returnvalue_2 (Actor|GetActorOfClass "/Game/Machines/BP_DeviceA1.BP_DeviceA1_C"))
  (if (Variables|/Game/Machines/BP_DeviceA1.BP_DeviceA1_C|GetDeviceActivated? _returnvalue_2)
    (bind _returnvalue_3 (Actor|GetActorOfClass "/Game/Gates/BP_GateA.BP_GateA_C"))
    (Default|PlayTimeline _returnvalue_3)))

(event OnComponentEndOverlap(PinkPlate_Collision)
  (params (OverlappedComponent :type Primitive%20Component%20Object%20Reference) (OtherActor :type Actor%20Object%20Reference) (OtherComp :type Primitive%20Component%20Object%20Reference) (OtherBodyIndex :type Integer))
  ;[1 0.2604 0.5964] Pink
  (Utilities|Casting|CastToBP_Holdable_ItemC OtherActor)
  (Rendering|Material|SetMaterial (Variables|Default|GetSM_PinkPlate) 0 "/Game/Materials/M_Grey.M_Grey")
  (bind _returnvalue (Actor|GetActorOfClass "/Game/Machines/BP_DeviceA1.BP_DeviceA1_C"))
  (Rendering|Material|SetMaterial (Variables|/Game/Machines/BP_DeviceA1.BP_DeviceA1_C|GetCylinder _returnvalue) 0 "/Game/Materials/M_Grey.M_Grey")
  (Variables|Default|SetPinkActivated? false)
  (bind _returnvalue_2 (Actor|GetActorOfClass "/Game/Gates/BP_GateA.BP_GateA_C"))
  (Default|ReverseTimeline _returnvalue_2))

(event OnComponentBeginOverlap(BluePlate_Collision)
  (params (OverlappedComponent :type Primitive%20Component%20Object%20Reference) (OtherActor :type Actor%20Object%20Reference) (OtherComp :type Primitive%20Component%20Object%20Reference) (OtherBodyIndex :type Integer) (bFromSweep :type Boolean) (SweepResult :type Hit%20Result%20Structure%20%28by%20ref%29))
  ;[0 0.5442 1] Blue
  (Utilities|Casting|CastToBP_Holdable_ItemC OtherActor)
  (Rendering|Material|SetMaterial (Variables|Default|GetSM_BluePlate) 0 "/Game/Materials/M_BlueGlow.M_BlueGlow")
  (bind _returnvalue (Actor|GetActorOfClass "/Game/BP_Lights.BP_Lights_C"))
  (Rendering|Components|Light|SetIntensity (Variables|/Game/BP_Lights.BP_Lights_C|GetPointLight1 _returnvalue) 1e+04))

(event OnComponentEndOverlap(BluePlate_Collision)
  (params (OverlappedComponent :type Primitive%20Component%20Object%20Reference) (OtherActor :type Actor%20Object%20Reference) (OtherComp :type Primitive%20Component%20Object%20Reference) (OtherBodyIndex :type Integer))
  ;[0 0.5442 1] Blue
  (Utilities|Casting|CastToBP_Holdable_ItemC OtherActor)
  (Rendering|Material|SetMaterial (Variables|Default|GetSM_BluePlate) 0 "/Game/Materials/M_Grey.M_Grey")
  (bind _returnvalue (Actor|GetActorOfClass "/Game/BP_Lights.BP_Lights_C"))
  (Rendering|Components|Light|SetIntensity (Variables|/Game/BP_Lights.BP_Lights_C|GetPointLight4 _returnvalue) 0.0))

(fn ConstructionScript)