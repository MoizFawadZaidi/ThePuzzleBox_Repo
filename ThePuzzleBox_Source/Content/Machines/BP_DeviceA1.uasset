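; BP_DeviceA1 is a puzzle machine that responds to a BP_Holdable_Item_BatteryA1 in its Box trigger and drives BP_GateA.
; Battery overlap sets DeviceActivated and plays the gate's timeline only if BP_Contraption's PinkActivated is true at that moment.
; Removing the battery clears the flag and reverses the gate timeline regardless of the contraption's state.
; The contraption and gate are found through GetActorOfClass lookups rather than stored references.
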(event OnComponentBeginOverlap(Box)
  (params (OverlappedComponent :type Primitive%20Component%20Object%20Reference) (OtherActor :type Actor%20Object%20Reference) (OtherComp :type Primitive%20Component%20Object%20Reference) (OtherBodyIndex :type Integer) (bFromSweep :type Boolean) (SweepResult :type Hit%20Result%20Structure%20%28by%20ref%29))
  (Utilities|Casting|CastToBP_Holdable_Item_BatteryA1 OtherActor)
  (Variables|Default|SetDeviceActivated? true)
  (bind _returnvalue (Actor|GetActorOfClass "/Game/Machines/BP_Contraption.BP_Contraption_C"))
  (if (Variables|/Game/Machines/BP_Contraption.BP_Contraption_C|GetPinkActivated? _returnvalue)
    (bind _returnvalue_2 (Actor|GetActorOfClass "/Game/Gates/BP_GateA.BP_GateA_C"))
    (Default|PlayTimeline _returnvalue_2)))

(event OnComponentEndOverlap(Box)
  (params (OverlappedComponent :type Primitive%20Component%20Object%20Reference) (OtherActor :type Actor%20Object%20Reference) (OtherComp :type Primitive%20Component%20Object%20Reference) (OtherBodyIndex :type Integer))
  (Utilities|Casting|CastToBP_Holdable_Item_BatteryA1 OtherActor)
  (Variables|Default|SetDeviceActivated? false)
  (bind _returnvalue (Actor|GetActorOfClass "/Game/Gates/BP_GateA.BP_GateA_C"))
  (Default|ReverseTimeline _returnvalue))

(fn ConstructionScript)