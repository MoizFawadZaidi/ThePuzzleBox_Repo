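; Puzzle device that toggles between green and blue on each interaction to control sliding doors B3 (blue) and C1 (green).
; A FlipFlop swaps glow material and colour flags, then acts only if pressure plate C3 has its sphere weight.
; Green also needs the contraption's RightGreenActivated to open C1, otherwise C1 closes.
; A battery C overlapping the box sets DeviceActivated, which the interaction never checks.
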(event OnComponentBeginOverlap(Box)
  (params (OverlappedComponent :type Primitive%20Component%20Object%20Reference) (OtherActor :type Actor%20Object%20Reference) (OtherComp :type Primitive%20Component%20Object%20Reference) (OtherBodyIndex :type Integer) (bFromSweep :type Boolean) (SweepResult :type Hit%20Result%20Structure%20%28by%20ref%29))
  (Utilities|Casting|CastToBP_Holdable_Item_BatteryC OtherActor)
  (Variables|Default|SetDeviceActivated? true))

(event OnComponentEndOverlap(Box)
  (params (OverlappedComponent :type Primitive%20Component%20Object%20Reference) (OtherActor :type Actor%20Object%20Reference) (OtherComp :type Primitive%20Component%20Object%20Reference) (OtherBodyIndex :type Integer))
  (Utilities|Casting|CastToBP_Holdable_Item_BatteryC OtherActor)
  (Variables|Default|SetDeviceActivated? false))

(event Custom|OPEN%20green%20CLOSE%20blue
  (bind _returnvalue (Actor|GetActorOfClass "/Game/SlidingDoors/BP_SlidingDoorC1.BP_SlidingDoorC1_C"))
  (Default|OpenDoors _returnvalue)
  (Utilities|IsValid (stale Custom|OPEN%20blue%20CLOSE%20green _returnvalue)
    (:Is%20Valid
      (Default|CloseDoors (stale Custom|OPEN%20blue%20CLOSE%20green _returnvalue)))))

(event Custom|OPEN%20blue%20CLOSE%20green
  (bind _returnvalue (Actor|GetActorOfClass "/Game/SlidingDoors/BP_SlidingDoorB3.BP_SlidingDoorB3_C"))
  (Default|OpenDoors _returnvalue)
  (Utilities|IsValid (stale Custom|OPEN%20green%20CLOSE%20blue _returnvalue)
    (:Is%20Valid
      (Default|CloseDoors (stale Custom|OPEN%20green%20CLOSE%20blue _returnvalue)))))

(event EventInteract
  (bind _cylinder (Variables|Default|GetCylinder))
  (Utilities|FlowControl|FlipFlop
    (:A
      (Rendering|Material|SetMaterial _cylinder 0 "/Game/Materials/M_GreenGlow.M_GreenGlow")
      (Variables|Default|SetGreenActivated? true)
      (Variables|Default|SetBlueActivated? false)
      (bind _returnvalue (Actor|GetActorOfClass "/Game/PressurePlates/BP_PressurePlateC3.BP_PressurePlateC3_C"))
      (if (Variables|/Game/PressurePlates/BP_PressurePlateC3.BP_PressurePlateC3_C|GetIsSphereWeight? _returnvalue)
        (bind _returnvalue_2 (Actor|GetActorOfClass "/Game/Machines/BP_Contraption.BP_Contraption_C"))
        (if (Variables|/Game/Machines/BP_Contraption.BP_Contraption_C|GetRightGreenActivated? _returnvalue_2)
          (CallFunction|OPENGreenCLOSEBlue)
          (else
            (bind _returnvalue_3 (Actor|GetActorOfClass "/Game/SlidingDoors/BP_SlidingDoorC1.BP_SlidingDoorC1_C"))
            (Default|CloseDoors _returnvalue_3)))))
    (:B
      (Rendering|Material|SetMaterial _cylinder 0 "/Game/Materials/M_BlueGlow.M_BlueGlow")
      (Variables|Default|SetBlueActivated? true)
      (Variables|Default|SetGreenActivated? false)
      (bind _returnvalue_4 (Actor|GetActorOfClass "/Game/PressurePlates/BP_PressurePlateC3.BP_PressurePlateC3_C"))
      (if (Variables|/Game/PressurePlates/BP_PressurePlateC3.BP_PressurePlateC3_C|GetIsSphereWeight? _returnvalue_4)
        (CallFunction|OPENBlueCLOSEGreen)))))

(fn ConstructionScript)