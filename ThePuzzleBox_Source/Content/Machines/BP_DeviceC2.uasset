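; BP_DeviceC2 is one of two battery-powered devices that together control BP_GateC.
; When a C2 battery enters its Box trigger, it sets Device2Activated, makes its Cylinder glow and plays the gate's timeline if BP_DeviceC1 is also active.
; Removing the battery clears the flag, restores the grey material and reverses the gate regardless of C1's state.
; It finds C1 and the gate by class lookup.
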(event OnComponentBeginOverlap(Box)
  (params (OverlappedComponent :type Primitive%20Component%20Object%20Reference) (OtherActor :type Actor%20Object%20Reference) (OtherComp :type Primitive%20Component%20Object%20Reference) (OtherBodyIndex :type Integer) (bFromSweep :type Boolean) (SweepResult :type Hit%20Result%20Structure%20%28by%20ref%29))
  (Utilities|Casting|CastToBP_Holdable_Item_BatteryC2 OtherActor)
  (Rendering|Material|SetMaterial (Variables|Default|GetCylinder) 0 "/Game/Materials/M_Glow.M_Glow")
  (Variables|Default|SetDevice2Activated? true)
  (bind _returnvalue (Actor|GetActorOfClass "/Game/Machines/BP_DeviceC1.BP_DeviceC1_C"))
  (if (Variables|/Game/Machines/BP_DeviceC1.BP_DeviceC1_C|GetDevice1Activated? _returnvalue)
    (bind _returnvalue_2 (Actor|GetActorOfClass "/Game/Gates/BP_GateC.BP_GateC_C"))
    (Default|PlayTimeline _returnvalue_2)))

(event OnComponentEndOverlap(Box)
  (params (OverlappedComponent :type Primitive%20Component%20Object%20Reference) (OtherActor :type Actor%20Object%20Reference) (OtherComp :type Primitive%20Component%20Object%20Reference) (OtherBodyIndex :type Integer))
  (Utilities|Casting|CastToBP_Holdable_Item_BatteryC2 OtherActor)
  (Rendering|Material|SetMaterial (Variables|Default|GetCylinder) 0 "/Game/Materials/M_Grey.M_Grey")
  (Variables|Default|SetDevice2Activated? false)
  (bind _returnvalue (Actor|GetActorOfClass "/Game/Gates/BP_GateC.BP_GateC_C"))
  (Default|ReverseTimeline _returnvalue))

(fn ConstructionScript)