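; BP_PressurePlateC3 is a pressure plate that detects a BP_SphereWeight actor.
; Box overlaps set the IsSphereWeight flag and switch the Plate material between blue glow and grey.
; The UpDown timeline moves the Cube component, playing from BeginPlay via MovePlateDown, independent of the overlaps.
; MovePlateUp reverses it but is not called here, and each overlap's GetActorOfClass result is unused.
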(event OnComponentBeginOverlap(Box)
  (params (OverlappedComponent :type Primitive%20Component%20Object%20Reference) (OtherActor :type Actor%20Object%20Reference) (OtherComp :type Primitive%20Component%20Object%20Reference) (OtherBodyIndex :type Integer) (bFromSweep :type Boolean) (SweepResult :type Hit%20Result%20Structure%20%28by%20ref%29))
  (Utilities|Casting|CastToBP_SphereWeight OtherActor)
  (Variables|Default|SetIsSphereWeight? true)
  (Rendering|Material|SetMaterial (Variables|Default|GetPlate) 0 "/Game/Materials/M_BlueGlow.M_BlueGlow")
  (Actor|GetActorOfClass "BP_PressurePlateC3_C"))

(event OnComponentEndOverlap(Box)
  (params (OverlappedComponent :type Primitive%20Component%20Object%20Reference) (OtherActor :type Actor%20Object%20Reference) (OtherComp :type Primitive%20Component%20Object%20Reference) (OtherBodyIndex :type Integer))
  (Utilities|Casting|CastToBP_SphereWeight OtherActor)
  (Variables|Default|SetIsSphereWeight? false)
  (Rendering|Material|SetMaterial (Variables|Default|GetPlate) 0 "/Game/Materials/M_Grey.M_Grey")
  (Actor|GetActorOfClass "BP_PressurePlateC3_C"))

(event Custom|Move%20Plate%20Down
  (bind _up_and_down_movement_track (Timeline|Up&Down Play)
    (:Update
      (Transformation|SetRelativeLocation (Variables|Default|GetCube) _up_and_down_movement_track false false))))

(event Custom|Move%20Plate%20Up
  (bind _up_and_down_movement_track (Timeline|Up&Down Reverse)
    (:Update
      (Transformation|SetRelativeLocation (Variables|Default|GetCube) _up_and_down_movement_track false false))))

(event EventBeginPlay
  (CallFunction|MovePlateDown))

(fn ConstructionScript)