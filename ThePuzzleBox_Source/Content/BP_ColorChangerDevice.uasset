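; BP_ColorChangerDevice is an interactable puzzle device that swaps the colours of two platforms on BP_QuadRotatePlatform.
; Each Interact alternates through a FlipFlop, finding the platform actor by class and switching the Owl and Coffee platform meshes between blue and green materials.
; The same toggle sets CorrectCombo, true when Owl is blue and Coffee is green, false otherwise.
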(event EventInteract
  (Utilities|FlowControl|FlipFlop
    (:A
      (bind _returnvalue (Actor|GetActorOfClass "/Game/RotatingPlatfomrs/BP_QuadRotatePlatform.BP_QuadRotatePlatform_C"))
      (Rendering|Material|SetMaterial (Variables|/Game/RotatingPlatfomrs/BP_QuadRotatePlatform.BP_QuadRotatePlatform_C|GetSM_OwlPlatform _returnvalue) 0 "/Game/Materials/M_Blue.M_Blue")
      (Rendering|Material|SetMaterial (Variables|/Game/RotatingPlatfomrs/BP_QuadRotatePlatform.BP_QuadRotatePlatform_C|GetSM_CoffeePlatform _returnvalue) 0 "/Game/Materials/M_Green.M_Green")
      (Variables|Default|SetCorrectCombo true))
    (:B
      (bind _returnvalue_2 (Actor|GetActorOfClass "/Game/RotatingPlatfomrs/BP_QuadRotatePlatform.BP_QuadRotatePlatform_C"))
      (Rendering|Material|SetMaterial (Variables|/Game/RotatingPlatfomrs/BP_QuadRotatePlatform.BP_QuadRotatePlatform_C|GetSM_OwlPlatform _returnvalue_2) 0 "/Game/Materials/M_Green.M_Green")
      (Rendering|Material|SetMaterial (Variables|/Game/RotatingPlatfomrs/BP_QuadRotatePlatform.BP_QuadRotatePlatform_C|GetSM_CoffeePlatform _returnvalue_2) 0 "/Game/Materials/M_Blue.M_Blue")
      (Variables|Default|SetCorrectCombo false))))

(fn ConstructionScript)